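; Fire bolt gameplay ability that launches homing projectiles at the target under the crosshair.
; On valid target data it commits, then turns the avatar through its combat component toward the hit location, or the camera direction when no actor is hit.
; It plays a sped-up attack montage, spawns pitch-overridden projectiles on the montage's FireBolt gameplay event, and ends when the montage completes, blends out or is interrupted.
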(event `self.K2_ActivateAbility`
  (bind (_asynctaskproxy _datahandle) (`TargetDataUnderCrosshair.CreateTargetDataUnderCrosshair` false)
    (:`ValidData`
      (bind (_bblockinghit _binitialoverlap _time _distance _location _impactpoint _normal _impactnormal _physmat _hitactor) (`GameplayStatics.BreakHitResult` (`AbilitySystemBlueprintLibrary.GetHitResultFromTargetData` _datahandle)))
      (set `self.TargetLocation` _location)
      (set `self.Hit Actor` _hitactor)
      (`self.K2_CommitAbility`)
      (bind _returnvalue (`AbyssBlueprintLibrary.BP_GetCombatComponentFromActor` (`self.GetAvatarActorFromActorInfo`))
        (:`Valid`
          (`/Engine/EditorBlueprintResources/StandardMacros.IsValid` (`self.Hit Actor`)
            (:`Is Valid`
              (`AbyssCombatComponentBase.SetFacingTarget` _returnvalue (`self.TargetLocation`)))
            (:`Is Not Valid`
              (`AbyssCombatComponentBase.SetFacingToCameraDirection` _returnvalue)))
          (`AbilityTask_PlayMontageAndWait.CreatePlayMontageAndWaitProxy` "None" "/Game/Abyss/Hero/AnimAssets/Abyss_Attack_Up_01_Seq_Montage.Abyss_Attack_Up_01_Seq_Montage" 3.0
            (:`then`
              (bind (_asynctaskproxy_2 _payload) (`AbilityTask_WaitGameplayEvent.WaitGameplayEvent` (struct :`TagName` "AbyssTags.Events.Montage.FireBolt") null)
                (:`EventReceived`
                  (if (`self.bDrawDebugs`)
                    (`KismetSystemLibrary.PrintString` (`KismetStringLibrary.Concat_StrStr` "rec:" (`KismetSystemLibrary.GetDisplayName` (`.Instigator` (break `GameplayEventData` _payload))))))
                  (`self.SpawnProjectiles` (`self.TargetLocation`) (struct) false 30.0 (`self.Hit Actor`)))))
            (:`OnCompleted`
              (`self.K2_EndAbility` :!label _label))
            (:`OnBlendOut`
              (goto _label))
            (:`OnInterrupted`
              (goto _label))
            (:`OnCancelled`
              (goto _label))))))))